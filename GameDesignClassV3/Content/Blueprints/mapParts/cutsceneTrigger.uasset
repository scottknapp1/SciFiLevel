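; Trigger actor that plays the end-of-level cinematic when the player overlaps its Er component.
; Any overlap sets IscutSceneGoing on GameModeMain, before the check that the overlapping actor is the player's BP_ThirdPersonCharacter.
; For the player, it creates and plays the EndlevelCinematic level sequence, then adds a BlackOut widget to the viewport after a fixed delay.
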(event OnComponentBeginOverlap(er)
  (params (OverlappedComponent :type Primitive%20Component%20Object%20Reference) (OtherActor :type Actor%20Object%20Reference) (OtherComp :type Primitive%20Component%20Object%20Reference) (OtherBodyIndex :type Integer) (bFromSweep :type Boolean) (SweepResult :type Hit%20Result%20Structure%20%28by%20ref%29))
  (bind _asgame_mode_main (Utilities|Casting|CastToGameModeMain (Game|GetGameMode)))
  (Variables|/Game/Blueprints/respawn/GameModeMain.GameModeMain_C|SetiscutSceneGoing _asgame_mode_main true)
  (bind _asbp_third_person_character (Utilities|Casting|CastToBP_ThirdPersonCharacter (Game|GetPlayerCharacter 0)))
  (if (== _asbp_third_person_character OtherActor)
    (bind _outactor (Sequencer|Player|CreateLevelSequencePlayer "/Game/CutScene/EndlevelCinematic.EndlevelCinematic"))
    (Sequencer|Player|Play (Variables|/Script/LevelSequence.LevelSequenceActor|GetSequencePlayer _outactor) :!class /Script/MovieScene.MovieSceneSequencePlayer)
    (Utilities|FlowControl|Delay 8.0)
    (bind _returnvalue (UserInterface|CreateWidget "/Game/Blueprints/UI/BlackOut.BlackOut_C"))
    (UserInterface|Viewport|AddtoViewport _returnvalue 0)))

(fn ConstructionScript)