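; Chest map part that unlocks the spell ability when the player interacts with it.
; A Box overlap with the third-person character enables input on the chest, and leaving the box disables it.
; Pressing interact while input is enabled shows the AbiltyUnlock widget, sets Havespell on GameModeMain, and destroys the chest.
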(event OnComponentBeginOverlap(Box)
  (params (OverlappedComponent :type Primitive%20Component%20Object%20Reference) (OtherActor :type Actor%20Object%20Reference) (OtherComp :type Primitive%20Component%20Object%20Reference) (OtherBodyIndex :type Integer) (bFromSweep :type Boolean) (SweepResult :type Hit%20Result%20Structure%20%28by%20ref%29))
  ;[1 1 1] inside range chest
  (Utilities|Casting|CastToBP_ThirdPersonCharacter OtherActor)
  (Input|EnableInput (Game|GetPlayerController 0)))

(event OnComponentEndOverlap(Box)
  (params (OverlappedComponent :type Primitive%20Component%20Object%20Reference) (OtherActor :type Actor%20Object%20Reference) (OtherComp :type Primitive%20Component%20Object%20Reference) (OtherBodyIndex :type Integer))
  ;[1 1 1] outside range chest
  (Utilities|Casting|CastToBP_ThirdPersonCharacter OtherActor)
  (Input|DisableInput (Game|GetPlayerController 0)))

(event Input|ActionEvents|InputActioninteract
  (params (Key :type Key%20Structure :default "None"))
  (:Pressed
    (bind _returnvalue (UserInterface|CreateWidget "/Game/Blueprints/UI/AbiltyUnlock.AbiltyUnlock_C"))
    (UserInterface|Viewport|AddtoViewport _returnvalue 0)
    (bind _asgame_mode_main (Utilities|Casting|CastToGameModeMain (Game|GetGameMode)))
    (Variables|/Game/Blueprints/respawn/GameModeMain.GameModeMain_C|Sethavespell _asgame_mode_main true)
    (Actor|DestroyActor)))

(fn ConstructionScript)