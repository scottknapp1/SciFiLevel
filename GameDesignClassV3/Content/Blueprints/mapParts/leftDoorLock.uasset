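; Left door lock map part that shows when the left side has been smashed and disappears once both sides are.
; Every tick it casts the game mode to GameModeMain and polls its SmashedLeft and Smashedright flags.
; SmashedLeft switches the static mesh material to Green, and Smashedright also being true then destroys the actor.
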(event EventTick
  (params (DeltaSeconds :type Float%20%28single-precision%29))
  (bind _asgame_mode_main (Utilities|Casting|CastToGameModeMain (Game|GetGameMode)))
  (if (== (Variables|/Game/Blueprints/respawn/GameModeMain.GameModeMain_C|GetsmashedLeft _asgame_mode_main) true)
    (Rendering|Material|SetMaterial (Variables|Default|GetStaticMesh) 0 "/Game/Material/green.green")
    (if (== (Variables|/Game/Blueprints/respawn/GameModeMain.GameModeMain_C|Getsmashedright _asgame_mode_main) true)
      (Actor|DestroyActor))))

(fn ConstructionScript)