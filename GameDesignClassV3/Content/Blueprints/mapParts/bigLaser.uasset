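; Laser hazard map part that fires a beam along its forward vector and destroys the player character on contact.
; Each tick a visibility line trace sets the beam's end to the hit point, or to the full Distance when nothing blocks it.
; An impact effect moves to the hit location and shows only while blocked.
; BeginPlay tints both beam and impact effects red.
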(event EventBeginPlay
  ;[1 1 1] set laser colour
  (Effects|Components|ParticleSystem|SetColorParameter (Variables|Default|Getlaser) "colour" "(R=0.950000,G=0.131159,B=0.085777,A=1.000000)")
  (Effects|Components|ParticleSystem|SetColorParameter (Variables|Default|GetlaserImpact) "colour" "(R=1.000000,G=0.121419,B=0.073650,A=1.000000)"))

(event EventTick
  (params (DeltaSeconds :type Float%20%28single-precision%29))
  (bind _returnvalue (Transformation|GetActorLocation))
  (bind _returnvalue_2 (Transformation|GetActorForwardVector))
  (bind _returnvalue_3 (Game|GetPlayerCharacter 0))
  (bind _distance (Variables|Default|Getdistance))
  (bind _returnvalue_4 (* _returnvalue_2 _distance))
  (bind _returnvalue_5 (+ _returnvalue _returnvalue_4))
  ;[1 1 1] draws laser and adjust length
  (Variables|Default|SetLaserEnd _returnvalue_5)
  (bind _outhit (Collision|LineTraceByChannel _returnvalue _returnvalue_5 "TraceTypeQuery1" false 0 "None"))
  (Variables|Default|SetwhosHit (.hitactor _outhit))
  (Variables|Default|SetbeingHit (.bblockinghit _outhit))
  (Variables|Default|SetHitLocation (.location _outhit))
  (Effects|Components|ParticleSystem|SetVectorParameter (Variables|Default|Getlaser) "laserEnd" (select (Variables|Default|GetbeingHit) (Variables|Default|GetHitLocation) (Variables|Default|GetLaserEnd)))
  (Rendering|SetVisibility (Variables|Default|GetlaserImpact) (Variables|Default|GetbeingHit) false)
  (Transformation|SetWorldLocation (Variables|Default|GetlaserImpact) (Variables|Default|GetHitLocation) false false)
  ;[1 1 1] kils player if laser hits
  (bind _asbp_third_person_character (Utilities|Casting|CastToBP_ThirdPersonCharacter _returnvalue_3))
  (if (== _asbp_third_person_character (Variables|Default|GetwhosHit))
    (Actor|DestroyActor _returnvalue_3)))

(fn ConstructionScript)