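; Power generator map part that animates its static mesh by stepping down its uniform world scale.
; Tick drives a chain of Delay nodes, each followed by a SetWorldScale3D fed by a vector lerp.
; Every lerp alpha is fixed at zero, so steps snap to their start scale and never reach the final smallest size.
; Tick keeps re-entering the first Delay, so the steps repeat and overlap.
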(event EventTick
  (params (DeltaSeconds :type Float%20%28single-precision%29))
  (Utilities|FlowControl|Delay 0.9)
  (Transformation|SetWorldScale3D (Variables|Default|GetStaticMesh) (Math|Vector|Lerp(Vector) "2.000000,2.000000,2.000000" "1.800000,1.800000,1.800000" 0.0))
  (Utilities|FlowControl|Delay 1.0)
  (Transformation|SetWorldScale3D (Variables|Default|GetStaticMesh) (Math|Vector|Lerp(Vector) "1.800000,1.800000,1.800000" "1.600000,1.600000,1.600000" 0.0))
  (Utilities|FlowControl|Delay 1.0)
  (Transformation|SetWorldScale3D (Variables|Default|GetStaticMesh) (Math|Vector|Lerp(Vector) "1.600000,1.600000,1.600000" "1.400000,1.400000,1.400000" 0.0))
  (Utilities|FlowControl|Delay 1.0)
  (Transformation|SetWorldScale3D (Variables|Default|GetStaticMesh) (Math|Vector|Lerp(Vector) "1.400000,1.400000,1.400000" "1.200000,1.200000,1.200000" 0.0))
  (Utilities|FlowControl|Delay 1.0)
  (Transformation|SetWorldScale3D (Variables|Default|GetStaticMesh) (Math|Vector|Lerp(Vector) "1.200000,1.200000,1.200000" "1.000000,1.000000,1.000000" 0.0)))

(fn ConstructionScript)