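; Pressure panel Blueprint, named for the reactor room, that drives a level sequence when something overlaps its collision component.
; Overlap begin turns the pad green and plays the sequence, while overlap end turns it red and plays the sequence in reverse.
; Each event creates a fresh sequence player rather than reusing one, and neither checks which actor overlapped.
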(event OnComponentBeginOverlap(collision)
  (params (OverlappedComponent :type Primitive%20Component%20Object%20Reference) (OtherActor :type Actor%20Object%20Reference) (OtherComp :type Primitive%20Component%20Object%20Reference) (OtherBodyIndex :type Integer) (bFromSweep :type Boolean) (SweepResult :type Hit%20Result%20Structure%20%28by%20ref%29))
  (Rendering|Material|SetMaterial (Variables|Default|Getpad) 0 "/Game/Material/green.green")
  (bind (_outactor _returnvalue) (Sequencer|Player|CreateLevelSequencePlayer (Variables|Default|Getsequence)))
  (Sequencer|Player|Play (Variables|/Script/LevelSequence.LevelSequenceActor|GetSequencePlayer _outactor) :!class /Script/MovieScene.MovieSceneSequencePlayer))

(event OnComponentEndOverlap(collision)
  (params (OverlappedComponent :type Primitive%20Component%20Object%20Reference) (OtherActor :type Actor%20Object%20Reference) (OtherComp :type Primitive%20Component%20Object%20Reference) (OtherBodyIndex :type Integer))
  (Rendering|Material|SetMaterial (Variables|Default|Getpad) 0 "/Game/Material/red.red")
  (bind _outactor (Sequencer|Player|CreateLevelSequencePlayer (Variables|Default|Getsequence)))
  (Class|MovieSceneSequencePlayer|PlayReverse (Variables|/Script/LevelSequence.LevelSequenceActor|GetSequencePlayer _outactor)))

(fn ConstructionScript)