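; Floor tile map part that drops out from under the player after a warning, then restores itself.
; When the player character overlaps the Box trigger, the static mesh switches to a red material as a warning.
; After a delay the actor is hidden and mesh collision is disabled, then a shorter delay brings back visibility, collision and a green material.
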(event OnComponentBeginOverlap(Box)
  (params (OverlappedComponent :type Primitive%20Component%20Object%20Reference) (OtherActor :type Actor%20Object%20Reference) (OtherComp :type Primitive%20Component%20Object%20Reference) (OtherBodyIndex :type Integer) (bFromSweep :type Boolean) (SweepResult :type Hit%20Result%20Structure%20%28by%20ref%29))
  (bind _returnvalue (Game|GetPlayerCharacter 0))
  ;[1 1 1] drops floor and set warning colour
  (Utilities|Casting|CastToBP_ThirdPersonCharacter _returnvalue)
  (if (== OtherActor _returnvalue)
    (Rendering|Material|SetMaterial (Variables|Default|GetStaticMesh) 0 "/Game/Material/red.red")
    (Utilities|FlowControl|Delay 5.0)
    (Rendering|SetActorHiddenInGame true)
    (Collision|SetCollisionEnabled (Variables|Default|GetStaticMesh) "NoCollision")
    (Utilities|FlowControl|Delay 2.0)
    (Rendering|SetActorHiddenInGame false)
    (Collision|SetCollisionEnabled (Variables|Default|GetStaticMesh) "QueryAndPhysics")
    (Rendering|Material|SetMaterial (Variables|Default|GetStaticMesh) 0 "/Game/Material/green.green")))

(fn ConstructionScript)