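; Switchable light Blueprint that shows its on or off state by turning its point light green or red.
; ToggleLight checks the Lighton flag and calls the matching on or off event, which sets the color and updates the flag.
; Turning on adds one to NumberOfclicks in GameModeMain and turning off subtracts one, so each toggle adjusts that shared count.
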(event Custom|turnLightOn
  ;[1 1 1] turn light on
  (Rendering|Components|Light|SetLightColor (Variables|Default|GetPointLight) "(R=0.092569,G=1.000000,B=0.033333,A=1.000000)" true)
  (Variables|Default|Setlighton? true)
  (bind _asgame_mode_main (Utilities|Casting|CastToGameModeMain (Game|GetGameMode)))
  (Variables|/Game/Blueprints/respawn/GameModeMain.GameModeMain_C|SetNumberOfclicks _asgame_mode_main (+ (Variables|/Game/Blueprints/respawn/GameModeMain.GameModeMain_C|GetNumberOfclicks _asgame_mode_main) 1)))

(event Custom|turnLightOff
  ;[1 1 1] turn light off
  (Rendering|Components|Light|SetLightColor (Variables|Default|GetPointLight) "(R=1.000000,G=0.012500,B=0.012500,A=1.000000)" true)
  (Variables|Default|Setlighton? false)
  (bind _asgame_mode_main (Utilities|Casting|CastToGameModeMain (Game|GetGameMode)))
  (Variables|/Game/Blueprints/respawn/GameModeMain.GameModeMain_C|SetNumberOfclicks _asgame_mode_main (+ (Variables|/Game/Blueprints/respawn/GameModeMain.GameModeMain_C|GetNumberOfclicks _asgame_mode_main) -1)))

(event Custom|ToggleLight
  ;[1 1 1] toggle light
  (if (Variables|Default|Getlighton?)
    (CallFunction|TurnLightOff)
    (else
      (CallFunction|TurnLighton))))

(fn ConstructionScript)