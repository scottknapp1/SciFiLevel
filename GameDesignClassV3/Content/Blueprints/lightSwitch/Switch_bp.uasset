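; Switch_bp is an interactable light switch that toggles a set of referenced lights.
; Overlapping its Box with BP_ThirdPersonCharacter enables player input on the switch, and leaving the box disables it.
; While input is enabled, pressing the interact action loops through the LightREF array and calls ToggleLight on each entry.
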(event OnComponentBeginOverlap(Box)
  (params (OverlappedComponent :type Primitive%20Component%20Object%20Reference) (OtherActor :type Actor%20Object%20Reference) (OtherComp :type Primitive%20Component%20Object%20Reference) (OtherBodyIndex :type Integer) (bFromSweep :type Boolean) (SweepResult :type Hit%20Result%20Structure%20%28by%20ref%29))
  ;[1 1 1] inside range switch
  (Utilities|Casting|CastToBP_ThirdPersonCharacter OtherActor)
  (Input|EnableInput (Game|GetPlayerController 0)))

(event OnComponentEndOverlap(Box)
  (params (OverlappedComponent :type Primitive%20Component%20Object%20Reference) (OtherActor :type Actor%20Object%20Reference) (OtherComp :type Primitive%20Component%20Object%20Reference) (OtherBodyIndex :type Integer))
  ;[1 1 1] outside range switch
  (Utilities|Casting|CastToBP_ThirdPersonCharacter OtherActor)
  (Input|DisableInput (Game|GetPlayerController 0)))

(event Input|ActionEvents|InputActioninteract
  (params (Key :type Key%20Structure :default "None"))
  ;[1 1 1] toggle light
  (:Pressed
    (bind _array_element (Utilities|Array|ForEachLoopwithBreak (Variables|Default|GetlightREF))
      (:LoopBody
        (Default|ToggleLight _array_element)))))

(fn ConstructionScript)