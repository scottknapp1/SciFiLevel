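; GameModeMain is a game mode that respawns the player at the latest saved spawn location after death.
; It stores the most recent login as MainPlayer, binds to its pawn's OnDestroyed on each restart, and restarts MainPlayer when that fires.
; UpdateRespawnLoc sets SpawnLoc, which the FindPlayerStart override returns when valid, falling back to a PlayerStart found by class.
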(event Custom|playerdied
  (params (DestroyedActor :type Actor%20Object%20Reference))
  ;[1 1 1] checks if player dies and respawns
  (Class|GameModeBase|RestartPlayer (Variables|Default|GetMainPlayer)))

(event EventPostLogin
  (params (NewPlayer :type Player%20Controller%20Object%20Reference))
  ;[1 1 1] checks if player is in game
  (bind _output_get (Variables|Default|SetMainPlayer NewPlayer))
  (Class|GameModeBase|RestartPlayer _output_get))

(event EventOnRestartPlayer
  (params (NewPlayer :type Controller%20Object%20Reference))
  ;[1 1 1] checks if player dies and respawns
  (Game|BindEventtoOnDestroyed (Pawn|GetControlledPawn NewPlayer) (delegate Custom|playerdied)))

(event EventUpdateRespawnLoc
  (params (NewLoc :type Actor%20Object%20Reference))
  ;[1 1 1] updates spawn loc
  (Variables|Default|SetspawnLoc NewLoc))

(fn ConstructionScript)

(fn FindPlayerStart
  (params (Player :type Controller%20Object%20Reference) (IncomingName :type String))
  (bind _spawnloc (Variables|Default|GetspawnLoc)
    (:then
      (return _spawnloc))
    (:else
      (bind _returnvalue (Actor|GetActorOfClass "/Script/Engine.PlayerStart"))
      (return _returnvalue))))